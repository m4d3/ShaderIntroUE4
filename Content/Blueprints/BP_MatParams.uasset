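; BP_MatParams is an actor that demonstrates animating material parameters at runtime on its static mesh.
; The construction script creates a dynamic instance of M_MatParameter and stores it as Material.
; On BeginPlay, a timeline ping-pongs endlessly, lerping the Color vector and TextureTiling scalar parameters.
; Each time the forward pass finishes, a FlipFlop swaps the Texture parameter between a noise and a grid texture.
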(event EventBeginPlay
  (bind _material (Variables|Default|GetMaterial))
  (bind _materialanimation (Variables|Default|GetMaterialAnimation))
  (bind (_direction _alpha) (Timeline|MaterialAnimation PlayFromStart)
    (:Update
      (Utilities|FlowControl|Sequence
        (:then_0
          (Rendering|Material|SetVectorParameterValue _material "Color" (Math|Color|Lerp(LinearColor) "(R=0.000000,G=0.873422,B=1.000000,A=1.000000)" "(R=1.000000,G=0.000000,B=0.912283,A=1.000000)" _alpha) :!class /Script/Engine.MaterialInstanceDynamic))
        (:then_1
          (Rendering|Material|SetScalarParameterValue _material "TextureTiling" (Math|Float|Lerp 0.25 5.0 _alpha) :!class /Script/Engine.MaterialInstanceDynamic))))
    (:Finished
      (switch Utilities|FlowControl|Switch|SwitchonETimelineDirection _direction
        (:Forward
          (Utilities|FlowControl|Sequence
            (:then_0
              (Utilities|FlowControl|FlipFlop
                (:A
                  (Rendering|Material|SetTextureParameterValue _material "Texture" "/Engine/MaterialTemplates/Textures/T_Noise01.T_Noise01"))
                (:B
                  (Rendering|Material|SetTextureParameterValue _material "Texture" "/Engine/EngineMaterials/Grid.Grid"))))
            (:then_1
              (Components|Timeline|ReversefromEnd _materialanimation))))
        (:Backward
          (Components|Timeline|PlayfromStart _materialanimation))))))

(event Collision|EventActorBeginOverlap
  (params (OtherActor :type Actor%20Object%20Reference)))

(event EventTick
  (params (DeltaSeconds :type Float%20%28single-precision%29)))

(fn ConstructionScript
  (bind _returnvalue (Rendering|Material|CreateDynamicMaterialInstance (Variables|Debug|GetStaticMeshComponent) 0 "/Game/Materials/M_MatParameter.M_MatParameter" :!class /Script/Engine.PrimitiveComponent))
  (Variables|Default|SetMaterial _returnvalue))